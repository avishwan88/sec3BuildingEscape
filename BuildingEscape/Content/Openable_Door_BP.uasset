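; Door actor that swings open and closed in response to the OnOpen and OnClose events of its OpenDoor component.
; A DoorMotion timeline scales the component's open angle into a yaw offset from the rotation stored at BeginPlay, and its event track plays a lock sound.
; Opening plays the timeline at a fixed rate, while closing reverses it at a rate derived from the component's close delay.
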(event `self.ReceiveBeginPlay`
  (set `self.Initial Rotation` (`self.K2_GetActorRotation`)))

(event `self.OpenDoor.OnOpen`
  (`TimelineComponent.SetPlayRate` (`self.DoorMotion`) 0.5)
  (bind (_direction _open_angle_percent) (`Timeline|DoorMotion` :!label _label)
    (:`Update`
      (`self.K2_SetActorRotation` (`KismetMathLibrary.ComposeRotators` (`self.Initial Rotation`) (`KismetMathLibrary.MakeRotator` 0.0 0.0 (* _open_angle_percent (`OpenDoor.OpenDoorAngle` (`self.OpenDoor`)))))))
    (:`Sound Timing`
      (`GameplayStatics.PlaySoundAtLocation` "/Game/Audio/door-lock.door-lock" (`self.K2_GetActorLocation`)))))

(event `self.OpenDoor.OnClose`
  (`TimelineComponent.SetPlayRate` (`self.DoorMotion`) (/ 1.0 (`OpenDoor.DoorCloseDelay` (`self.OpenDoor`))))
  (goto _label :!via `Reverse`))

(fn `UserConstructionScript`)